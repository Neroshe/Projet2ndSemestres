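; Overlap is a scripted scenario trigger that brings an AI actor into the scene when the first-person player enters its box.
; On BeginPlay it caches the world location of an arrow component as the spawn point.
; When the player overlaps the box, it teleports the referenced IaScénario actor to that point, destroys itself so it fires once, and tells the AI to start its MoveTo.
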(event `self.ReceiveBeginPlay`
  (set `self.spawn ia scenario` (`SceneComponent.K2_GetComponentLocation` (`self.Arrow spawn actor`))))

(event `self.Box.OnComponentBeginOverlap`
  (params (OverlappedComponent :type "PrimitiveComponent Object Reference") (OtherActor :type "Actor Object Reference") (OtherComp :type "PrimitiveComponent Object Reference") (OtherBodyIndex :type Integer) (bFromSweep :type Boolean) (SweepResult :type "HitResult Structure (by ref)"))
  (cast `/Game/FirstPerson/Blueprints/BP_FirstPersonCharacter` OtherActor)
  (`self.K2_SetActorLocation` (`self.ia_scénario`) (`self.spawn ia scenario`) false false)
  (`self.K2_DestroyActor`)
  (`/Game/Blueprints/scenario/BP_IA_Scnario.move to` (`self.ia_scénario`)))

(fn `UserConstructionScript`)